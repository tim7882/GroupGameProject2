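; BP_BounceTyre is a bounce pad that launches any Character overlapping its BounceArea.
; It treats LaunchVelocity as a target offset rotated with the actor, converting it to a launch vector with SuggestProjectileVelocityCustomArc.
; Flags optionally zero the character's velocity before launch and snap it above the pad afterwards.
; When DrawEditorLines is set, the construction script predicts the flight path and builds a chain of arrow components to preview the arc.
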(event `self.Bounce Area.OnComponentBeginOverlap`
  (params (OverlappedComponent :type "PrimitiveComponent Object Reference") (OtherActor :type "Actor Object Reference") (OtherComp :type "PrimitiveComponent Object Reference") (OtherBodyIndex :type Integer) (bFromSweep :type Boolean) (SweepResult :type "HitResult Structure (by ref)"))
  (bind _ascharacter (cast `Character` OtherActor))
  (bind _output_get (set `self.Character` _ascharacter))
  (if (`self.IgnoreCharacterVelocity`)
    (set `MovementComponent.Velocity` (0.0 0.0 0.0) (`Character.CharacterMovement` (`self.Character`))))
  (bind _launchvelocity (`self.calc launch velocity`))
  (`Character.LaunchCharacter` _output_get _launchvelocity false false)
  (if (`self.Adjust Character Position`)
    (`self.K2_SetActorLocation` (`self.Character`) (+ (`self.K2_GetActorLocation`) (0.0 0.0 100.0)) false false)))

(fn `calc launch velocity`
  (returns (LaunchVelocity :type "Vector Structure"))
  (bind _outlaunchvelocity (`GameplayStatics.SuggestProjectileVelocity_CustomArc` (0.0 0.0 0.0) (`KismetMathLibrary.GreaterGreater_VectorRotator` (`self.Launch Velocity`) (`self.K2_GetActorRotation`))))
  (return _outlaunchvelocity))

(fn `create launch arc`
  (params (LaunchVelocity :type "Vector Structure"))
  (bind (_outhit _outpathpositions) (`GameplayStatics.Blueprint_PredictProjectilePath_ByObjectType` :`StartPos` (+ (`self.K2_GetActorLocation`) (0.0 0.0 10.0)) :`LaunchVelocity` LaunchVelocity :`ProjectileRadius` 2.0 :`ObjectTypes` (`|MakeArray` "ObjectTypeQuery1" :!type "EObjectTypeQuery Enum") :`MaxSimTime` 20.0))
  (`self.CreateArkFromPositionArray` _outpathpositions))

(fn `CreateArkFromPositionArray`
  (params (Positions :type "Array of Vector Structure (by ref)"))
  (for (_array_element _array_index) Positions
    (if (!= _array_index 0)
      (bind _returnvalue (`AddComponent|NODE_AddArrowComponent-1` :`bManualAttachment` true :`RelativeTransform` (`self.make transform` _array_element (`|GetArrayItem` Positions (+ _array_index -1)))))
      (set `ArrowComponent.ArrowSize` 0.5 _returnvalue))))

(fn `UserConstructionScript`
  (if (`self.Draw Editor Lines`)
    (bind _launchvelocity (`self.calc launch velocity`))
    (`self.create launch arc` _launchvelocity)))