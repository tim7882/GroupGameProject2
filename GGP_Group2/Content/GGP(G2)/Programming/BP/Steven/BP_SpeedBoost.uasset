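; Speed boost pad that launches the player cube along its arrow and temporarily raises its walk speed.
; On box overlap it teleports the player to its scene point, locks movement and uses negative ground friction during the short launch, then restores both.
; A parallel delay resets movement values after the boost, and a timer-polled CanDash check after the launch can trigger the same reset.
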(event `self.ReceiveTick`
  (params (DeltaSeconds :type "Float (single-precision)")))

(event `self.Box.OnComponentBeginOverlap`
  (params (OverlappedComponent :type "PrimitiveComponent Object Reference") (OtherActor :type "Actor Object Reference") (OtherComp :type "PrimitiveComponent Object Reference") (OtherBodyIndex :type Integer) (bFromSweep :type Boolean) (SweepResult :type "HitResult Structure (by ref)"))
  (bind _as_new_player_cube_bp (`self.As New Player Cube BP`))
  ;[1 0.5496 0.07997] check if player is on the ground
  (bind _asnew_player_cube_bp (cast `/Game/GGP(G2)/Programming/New_PlayerCube_BP` OtherActor))
  (bind _output_get (set `self.As New Player Cube BP` _asnew_player_cube_bp))
  (set `/Game/GGP(G2)/Programming/New_PlayerCube_BP.Max Walk Speed` (`/Game/GGP(G2)/Programming/New_PlayerCube_BP.Max Walk Speed` _output_get) _output_get)
  (`SceneComponent.K2_SetWorldLocation` (`Actor.RootComponent` _output_get) (`SceneComponent.K2_GetComponentLocation` (`self.Scene`)) false true)
  (`|ExecutionSequence`
    (:`then_0`
      ;[1 0.5496 0.07997] locks player in a path
      (set `/Game/GGP(G2)/Programming/New_PlayerCube_BP.can move` false _as_new_player_cube_bp)
      (set `CharacterMovementComponent.GroundFriction` -10.0 (`Character.CharacterMovement` _as_new_player_cube_bp))
      (`Character.LaunchCharacter` _as_new_player_cube_bp (* (`SceneComponent.GetForwardVector` (`self.Arrow`)) 3000.0) true false)
      (`KismetSystemLibrary.Delay` 0.8)
      (set `CharacterMovementComponent.GroundFriction` (`/Game/GGP(G2)/Programming/New_PlayerCube_BP.Ground Friction` _as_new_player_cube_bp) (`Character.CharacterMovement` _as_new_player_cube_bp))
      (set `/Game/GGP(G2)/Programming/New_PlayerCube_BP.can move` true _as_new_player_cube_bp)
      (`self.check if player is moving`))
    (:`then_1`
      ;[1 0.5496 0.07997] add speed to the player
      (set `CharacterMovementComponent.MaxWalkSpeed` 1500.0 (`Character.CharacterMovement` _output_get))
      (`KismetSystemLibrary.Delay` 5.0)
      (`/Game/GGP(G2)/Programming/New_PlayerCube_BP.Reset Movement Value` _output_get :!label _label))))

(event `check if player is moving`
  ;[1 0.5496 0.07997] add speed to the player
  (if (`/Game/GGP(G2)/Programming/New_PlayerCube_BP.can dash` (stale `self.Box.OnComponentBeginOverlap` _output_get))
    (goto _label)
    (else
      (`KismetSystemLibrary.K2_SetTimerDelegate` (delegate `check if player is moving`) 1.0 true))))

(fn `UserConstructionScript`)